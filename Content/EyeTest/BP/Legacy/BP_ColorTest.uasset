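; Legacy color blindness test actor that runs a ten-plate number-reading session on BeginPlay and tallies correct answers.
; It shows one ColorTest component at a time and binds to the NumberEntered dispatcher of the KeyPad_UI widget on its KeyPad component.
; CheckedNumber compares input to the current plate's first component tag, then advances.
; After the last plate it prints the score in Korean and destroys itself.
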(event `self.ReceiveBeginPlay`
  (`self.Start Color Test`))

(event `Start Color Test`
  (`self.Session`))

(fn `Array`
  (returns (Output_Get :type "Array of StaticMeshComponent Object Reference"))
  (bind _output_get (set `self.EyeTestArray` (`|MakeArray` (`self.ColorTest01`) (`self.ColorTest02`) (`self.ColorTest03`) (`self.ColorTest04`) (`self.ColorTest05`) (`self.ColorTest06`) (`self.ColorTest07`) (`self.ColorTest08`) (`self.ColorTest09`) (`self.ColorTest10`))))
  (return _output_get))

(fn `Checked Number`
  (params (Number :type String) (Keypad :type "/Game/EyeTest/Widget/Keyboard/KeyPad_UI Object Reference"))
  (bind _currentindex (`self.CurrentIndex`))
  (bind _key_pad_ui (`self.Key Pad UI`))
  (if (`KismetStringLibrary.EqualEqual_StrStr` Number (`KismetTextLibrary.Conv_TextToString` (`KismetTextLibrary.Conv_NameToText` (`|GetArrayItem` (`ActorComponent.ComponentTags` (`|GetArrayItem` (`self.EyeTestArray`) (`self.CurrentIndex`)))))))
    (set `self.Correct?` true)
    (bind _result (`/Engine/EditorBlueprintResources/StandardMacros.IncrementInt` (`self.Correct Index`))
      (:`  `
        (set `self.Correct Index` _result)
        (`KismetSystemLibrary.PrintString` "Correct")
        (set `/Game/EyeTest/Widget/Keyboard/KeyPad_UI.CurrentNumber` "" _key_pad_ui)))
    (else
      (set `self.Correct?` false)
      (`KismetSystemLibrary.PrintString` "InCorrect")
      (set `/Game/EyeTest/Widget/Keyboard/KeyPad_UI.CurrentNumber` "" _key_pad_ui)))
  (`/Engine/EditorBlueprintResources/StandardMacros.IncrementInt` _currentindex
    (:`  `
      (if (> _currentindex 9)
        (`KismetSystemLibrary.PrintString` (`KismetStringLibrary.Concat_StrStr` "점수 : " (`KismetStringLibrary.Conv_IntToString` (`self.Correct Index`)) " / 색맹 검사 종료"))
        (`self.K2_DestroyActor`)
        (else
          (`self.Set Visibility` (`self.EyeTestArray`)))))))

(fn `Entered Number`
  (bind _askey_pad_ui (cast `/Game/EyeTest/Widget/Keyboard/KeyPad_UI` (`WidgetComponent.GetUserWidgetObject` (`self.KeyPad`))))
  (bind _output_get (set `self.Key Pad UI` _askey_pad_ui))
  (add `/Game/EyeTest/Widget/Keyboard/KeyPad_UI.NumberEntered` _output_get (`|CreateDelegate` :!event `Checked Number`)))

(fn `Session`
  (bind _output_get (`self.Array`))
  (`self.Set Visibility` _output_get)
  (`self.Set Test`))

(fn `Set Test`
  (`self.Entered Number`))

(fn `Set Visibility`
  (params (Array :type "Array of StaticMeshComponent Object Reference"))
  (for _array_element Array
    (`SceneComponent.SetVisibility` _array_element false false))
  (`SceneComponent.SetVisibility` (`|GetArrayItem` Array (`self.CurrentIndex`)) true false))

(fn `UserConstructionScript`)